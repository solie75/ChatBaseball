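; Player controller that passes ball input from the WBP_InputBall widget to BP_GameMode for calculation.
; On BeginPlay, when the remote role is not None, it waits briefly, finds the first top-level input widget, binds a message callback and asks the game mode to update the widget's data.
; OnSendBallToServer has the game mode calculate the submitted ball, then update the widget again, using direct GetGameMode casts.
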(event `self.ReceiveBeginPlay`
  (if (not (`|EnumEquality` (`self.GetRemoteRole`) "ROLE_None"))
    (`KismetSystemLibrary.Delay` 0.5)
    (bind _foundwidgets (`WidgetBlueprintLibrary.GetAllWidgetsOfClass` "/Game/Widget/WBP_InputBall.WBP_InputBall_C"))
    (bind _output_get (set `self.Widget` (`|GetArrayItem` _foundwidgets)))
    (bind _aswbp_input_ball (cast `/Game/Widget/WBP_InputBall` _output_get))
    (`|ExecutionSequence`
      (:`then_0`
        (add `/Game/Widget/WBP_InputBall.SetMessageToUserController` _aswbp_input_ball (`|CreateDelegate` :!event `OnSendBallToServer`)))
      (:`then_1`
        (bind _asbp_game_mode (cast `/Game/BP/BP_GameMode` (`GameplayStatics.GetGameMode`)))
        (`/Game/BP/BP_GameMode.UpdateWidgetData` _asbp_game_mode _aswbp_input_ball)))))

(event `OnSendBallToServer`
  (params (InputBall :type String))
  (bind _asbp_game_mode (cast `/Game/BP/BP_GameMode` (`GameplayStatics.GetGameMode`)))
  (`/Game/BP/BP_GameMode.CalculateBall` _asbp_game_mode InputBall)
  (bind _aswbp_input_ball (cast `/Game/Widget/WBP_InputBall` (`self.Widget`)))
  (`/Game/BP/BP_GameMode.UpdateWidgetData` _asbp_game_mode _aswbp_input_ball))

(fn `UserConstructionScript`)