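; Game mode that runs scoring for an inning-based number-baseball style game between the player and a server.
; CalculateBall adds strikes and balls from CalculateStrike, ending the inning on three cumulative strikes, an out, or three tries.
; Three strikes credit a player win regardless of turn, and each inning end resets counts and flips offense/defense.
; UpdateWidgetData writes inning, scores and turn to a widget, deriving server score from innings minus player wins.
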(event `CalculateBall`
  (params (InputBall :type String))
  (bind _returnvalue (`UmpireBPLibrary.CalculateStrike` InputBall))
  (set `self.TryCount` (+ 1 (`self.TryCount`)))
  (bind _output (`|GetArrayItem` _returnvalue))
  (set `self.StrikeCount` (+ (`self.StrikeCount`) _output))
  (if (>= (`self.StrikeCount`) 3)
    (set `self.PlayerWinCount` (+ (`self.PlayerWinCount`) 1))
    (set `self.IningCount` (+ (`self.IningCount`) 1) :!label _label)
    (set `self.TryCount` 0)
    (set `self.StrikeCount` 0)
    (set `self.BallCount` 0)
    (set `self.IsPlayerTurn` (not (`self.IsPlayerTurn`)))
    (else
      (bind _output_2 (`|GetArrayItem` _returnvalue 1))
      (set `self.BallCount` (+ (`self.BallCount`) _output_2))
      (if (== (+ _output_2 _output) 0)
        (goto _label)
        (elif (>= (`self.TryCount`) 3)
          (goto _label))))))

(event `UpdateWidgetData`
  (params (Widget :type "/Game/Widget/WBP_InputBall Object Reference"))
  (bind _textblock_isplayerturn (`/Game/Widget/WBP_InputBall.TextBlock_IsPlayerTurn` Widget))
  (set `TextBlock.Text` (`KismetTextLibrary.Conv_StringToText` (`KismetStringLibrary.Concat_StrStr` "Ining " ": " (`KismetStringLibrary.Conv_IntToString` (+ (`self.IningCount`) 1)))) (`/Game/Widget/WBP_InputBall.TextBlock_IningCount` Widget))
  (set `TextBlock.Text` (`KismetTextLibrary.Conv_StringToText` (`KismetStringLibrary.Concat_StrStr` "Plalyer Score " ": " (`KismetStringLibrary.Conv_IntToString` (`self.PlayerWinCount`)))) (`/Game/Widget/WBP_InputBall.TextBlock_Player` Widget))
  (set `TextBlock.Text` (`KismetTextLibrary.Conv_StringToText` (`KismetStringLibrary.Concat_StrStr` "Server Score " ": " (`KismetStringLibrary.Conv_IntToString` (- (`self.IningCount`) (`self.PlayerWinCount`))))) (`/Game/Widget/WBP_InputBall.TextBlock_Server` Widget))
  (if (`self.IsPlayerTurn`)
    (set `TextBlock.Text` "Offense" _textblock_isplayerturn)
    (else
      (set `TextBlock.Text` "Defense" _textblock_isplayerturn))))

(fn `UserConstructionScript`)